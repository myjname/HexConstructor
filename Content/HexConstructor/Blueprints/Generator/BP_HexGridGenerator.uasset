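; Hex map generator actor that builds an editable-height grid of big hex tiles from a grid size and height array.
; Instanced meshes draw big tiles scaled in Z, small tiles on top and patch tiles at three-tile junctions.
; Neighbour maps update patches on height edits, hiding them far below unless all three heights match.
; Line traces gate edits, Tick animates the selection marker, and GetMapHeights reads heights back from instance scales.
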(event `self.ReceiveBeginPlay`)

(event `GenerateHexGrid`
  (params (GridSize :type "IntPoint Structure") (MapHeights :type "Array of Integer"))
  (bind _gridsize_x (break `IntPoint` (`self.GridSize`)))
  (bind (_gridsize_x_2 _gridsize_y) (break `IntPoint` (`self.GridSize`)))
  (bind (_gridsize_x_3 _gridsize_y_2) (break `IntPoint` (`self.GridSize`)))
  (bind _curtile (`self.CurTile`))
  (bind _gridsize_x_4 (break `IntPoint` (`self.GridSize`)))
  (bind _hexpatchessize_x (break `IntPoint` (`self.HexPatchesSize`)))
  (bind _curtile_2 (`self.CurTile`))
  (bind (_gridsize_x_5 _gridsize_y_3) (break `IntPoint` (`self.GridSize`)))
  (bind _gridsize_x_6 (break `IntPoint` (`self.GridSize`)))
  (bind (_x _y _z) (break `IntVector` (`self.NeighbourHexes`)))
  (bind (_x_2 _y_2 _z_2) (break `IntVector` (`self.NeighbourHexes`)))
  (bind (_x_3 _y_3 _z_3) (break `IntVector` (`self.NeighbourHexes`)))
  (bind (_x_4 _y_4 _z_4) (break `IntVector` (`self.NeighbourHexes`)))
  (bind _returnvalue (- _gridsize_y 1))
  (bind _returnvalue_2 (* (`self.BigHexGridOffset`) (`self.CurColumn`)))
  (bind _returnvalue_3 (* (`self.BigHexGridOffset`) (- _gridsize_x_2 1)))
  (bind _returnvalue_4 (!= (mod (`self.CurTile`) 2) 0))
  (bind _returnvalue_5 (/ (+ (`self.CurTile`) 1) 2))
  (bind _returnvalue_6 (+ (+ (/ (`self.CurTile`) 2) _gridsize_x) (`self.CurRow`)))
  (bind _returnvalue_7 (+ _returnvalue_5 (* (/ (`self.CurRow`) 2) 2)))
  (bind _returnvalue_8 (- (`KismetMathLibrary.MakeVector` (select `bool` (== (mod (`self.CurRow`) 2) 1) :`false` _returnvalue_2 :`true` (+ _returnvalue_2 (/ (`self.BigHexGridOffset`) 2.0))) (* (* (`self.BigHexRadius`) 1.5) (`self.CurRow`))) (`self.HexGridOffset`)))
  (set `self.GridSize` GridSize)
  ;[0.15 0.15 0.15 0.5 72] Generate hex grids
  (set `self.Map Heights` MapHeights)
  (`|ExecutionSequence`
    (:`then_0`
      (`|ExecutionSequence`
        (:`then_0`
          (set `self.NumberOfBigTiles` (* _gridsize_x_3 _gridsize_y_2))
          (set `self.BigHexDiameter` (* (`self.BigHexRadius`) 2.0))
          (set `self.BigHexGridOffset` (* (`self.BigHexRadius`) (`KismetMathLibrary.Sqrt` 3.0)))
          (for _index (range 6)
            (`KismetArrayLibrary.Array_Add` (`self.SmallHexOffsets`) (`KismetMathLibrary.RotateAngleAxis` (`KismetMathLibrary.MakeVector` (/ (`self.BigHexGridOffset`) 3.0)) (* _index 60) (0.0 0.0 1.0)))))
        (:`then_1`
          (set `self.HexGridOffset` (* (`KismetMathLibrary.MakeVector` (select `bool` (== (mod _returnvalue 2) 1) :`false` _returnvalue_3 :`true` (+ _returnvalue_3 (/ (`self.BigHexGridOffset`) 2.0))) (* (* (`self.BigHexRadius`) 1.5) _returnvalue)) 0.5))
          (`KismetMaterialLibrary.SetVectorParameterValue` "/Game/HexConstructor/Art/Materials/GeneralMPC/MPC_HexGrid.MPC_HexGrid" "Offset" (`KismetMathLibrary.MakeColor` (.x (`self.HexGridOffset`)) (.y (`self.HexGridOffset`)) (.z (`self.HexGridOffset`)) 0.0))
          (for _index_2 (range (`self.NumberOfBigTiles`))
            (set `self.CurTile` _index_2)
            (set `self.CurColumn` (mod _curtile_2 _gridsize_x_4))
            (set `self.CurRow` (/ _curtile_2 _gridsize_x_4))
            (bind _returnvalue_9 (`InstancedStaticMeshComponent.AddInstance` (`self.ISM_BigHexTiles`) (`KismetMathLibrary.MakeTransform` _returnvalue_8 (struct) (`KismetMathLibrary.MakeVector` 1.0 1.0 (`KismetMathLibrary.Conv_IntToDouble` (`|GetArrayItem` (`self.Map Heights`) (`self.CurTile`))))) false))
            (`BlueprintMapLibrary.Map_Add` (`self.BigToSmallNeighbours`) _returnvalue_9 (make `/Game/HexConstructor/Blueprints/Structures/SInt32Array` (`|MakeArray`)))
            (for (_array_element _array_index) (`self.SmallHexOffsets`)
              (`InstancedStaticMeshComponent.SetCustomDataValue` (`self.ISM_BigHexTiles`) _returnvalue_9 _array_index -1.0 false)
              (`InstancedStaticMeshComponent.AddInstance` (`self.ISM_SmallHexTiles`) (`KismetMathLibrary.MakeTransform` (+ (+ _array_element _returnvalue_8) (`KismetMathLibrary.MakeVector` 0.0 0.0 (+ (* (`self.BigHexHeight`) (`self.InitialHeight`)) 1.0)))) false))))))
    (:`then_1`
      (`|ExecutionSequence`
        (:`then_0`
          (bind _output_get (set `self.HexPatchesSize` (make `IntPoint` (* (- _gridsize_x_5 1) 2) (- _gridsize_y_3 1))))
          (bind (_x_5 _y_5) (break `IntPoint` _output_get))
          (set `self.HexPatchesNum` (* _x_5 _y_5)))
        (:`then_1`
          (for _index_3 (range (`self.HexPatchesNum`))
            (set `self.CurTile` _index_3)
            (set `self.CurColumn` (mod _curtile _hexpatchessize_x))
            (set `self.CurRow` (/ _curtile _hexpatchessize_x))
            (set `self.NeighbourHexes` (select `bool` (select `bool` (== (mod (`self.CurRow`) 2) 0) :`false` (not _returnvalue_4) :`true` _returnvalue_4) :`false` (make `IntVector` _returnvalue_7 (+ _returnvalue_7 1) (+ (+ _returnvalue_5 _gridsize_x_6) (`self.CurRow`))) :`true` (make `IntVector` (+ _returnvalue_5 (`self.CurRow`)) _returnvalue_6 (+ _returnvalue_6 1))))
            (`|ExecutionSequence`
              (:`then_0`
                (set `self.AvgNeighbourHexesHeight` 0.0)
                (set `self.MidNeightbourLocation` (0.0 0.0 0.0))
                (for _array_element_2 (`|MakeArray` _x_4 _y_4 _z_4)
                  (set `self.MidNeightbourLocation` (+ (.location (`InstancedStaticMeshComponent.GetInstanceTransform` (`self.ISM_BigHexTiles`) _array_element_2 false)) (`self.MidNeightbourLocation`)))
                  (set `self.AvgNeighbourHexesHeight` (+ (`self.AvgNeighbourHexesHeight`) (.z (.scale (`InstancedStaticMeshComponent.GetInstanceTransform` (`self.ISM_BigHexTiles`) _array_element_2 false)))))))
              (:`then_1`
                (set `self.HeightEqual` true)
                (for _array_element_3 (`|MakeArray` _x _y _z)
                  (set `self.HeightEqual` (and (`self.HeightEqual`) (!= (`self.AvgNeighbourHexesHeight`) (.z (.scale (`InstancedStaticMeshComponent.GetInstanceTransform` (`self.ISM_BigHexTiles`) _array_element_3 false))))))))
              (:`then_2`
                (bind _output_get_2 (set `self.MidNeightbourLocation` (+ (/ (`self.MidNeightbourLocation`) 3.0) (`KismetMathLibrary.MakeVector` 0.0 0.0 (select `bool` (`self.HeightEqual`) :`false` -20000.0 :`true` (+ (* (`self.BigHexHeight`) (`self.InitialHeight`)) 1.0))))))
                (bind _returnvalue_10 (`InstancedStaticMeshComponent.AddInstance` (`self.ISM_SmallHexTiles`) (`KismetMathLibrary.MakeTransform` _output_get_2) false))
                (`BlueprintMapLibrary.Map_Add` (`self.SmallToBigNeighbours`) _returnvalue_10 (make `/Game/HexConstructor/Blueprints/Structures/SInt32Array` (`|MakeArray` _x_2 _y_2 _z_2)))
                (for _array_element_4 (`|MakeArray` _x_3 _y_3 _z_3)
                  (bind _output_get_3 (set `self.TempArray` (`.Array_3_0A781E194A4035A470EF75B61B08CBCF` (break `/Game/HexConstructor/Blueprints/Structures/SInt32Array` (`BlueprintMapLibrary.Map_Find` (`self.BigToSmallNeighbours`) _array_element_4)))))
                  (`KismetArrayLibrary.Array_Add` _output_get_3 _returnvalue_10)
                  (`BlueprintMapLibrary.Map_Add` (`self.BigToSmallNeighbours`) _array_element_4 (make `/Game/HexConstructor/Blueprints/Structures/SInt32Array` (`self.TempArray`))))))))
        (:`then_2`
          ;; Update for load save
          (for _index_4 (range (`InstancedStaticMeshComponent.GetInstanceCount` (`self.ISM_BigHexTiles`)))
            (`self.UpdateSmallTilesHeight` _index_4 (+ (* (.z (.scale (`InstancedStaticMeshComponent.GetInstanceTransform` (`self.ISM_BigHexTiles`) _index_4 false))) (`self.BigHexHeight`)) 1.0))))))
    (:`then_2`
      (`self.SetActorTickEnabled` true))))

(event `UpdateBigTilesHeight`
  (params (TileIndex :type Integer) (Scale :type "Float (double-precision)"))
  (bind _returnvalue (/ (`self.BigHexGridOffset`) 3.0))
  (bind _returnvalue_2 (+ (.z (.scale (`InstancedStaticMeshComponent.GetInstanceTransform` (`self.ISM_BigHexTiles`) TileIndex false))) (* Scale (`self.HeightScaleStep`))))
  ;[0.15 0.15 0.15 0.5 72] Change height of tile in grid
  (`|ExecutionSequence`
    (:`then_0`
      (set `self.CanChangeHeight` true)
      (for _array_element (`self.CoordiantesForChechTrace`)
        (bind _returnvalue_3 (- _array_element (make `IntPoint` 2 2)))
        (bind _returnvalue_4 (* _returnvalue (`.X` (break `IntPoint` _returnvalue_3))))
        (bind _returnvalue_5 (* (+ (`KismetMathLibrary.MakeVector` (select `bool` (!= (mod (`.Y` (break `IntPoint` _returnvalue_3)) 2) 0) :`false` _returnvalue_4 :`true` (+ _returnvalue_4 (/ _returnvalue 2.0))) (* (* (/ (`self.BigHexRadius`) 1.5) 0.75) (`.Y` (break `IntPoint` _returnvalue_3)))) (.location (`InstancedStaticMeshComponent.GetInstanceTransform` (`self.ISM_BigHexTiles`) TileIndex true))) (1.0 1.0 0.0)))
        (bind (_outhit _returnvalue_6) (`KismetSystemLibrary.LineTraceSingle` :`Start` (+ _returnvalue_5 (0.0 0.0 5000.0)) :`End` _returnvalue_5 :`TraceChannel` "TraceTypeQuery5" :`DrawTime` 0.3))
        (set `self.CanChangeHeight` (and (not _returnvalue_6) (`self.CanChangeHeight`)))))
    (:`then_1`
      (if (`self.CanChangeHeight`)
        (if (or (> Scale 0.0) (> _returnvalue_2 (* (`self.HeightScaleStep`) 2.0)))
          (`InstancedStaticMeshComponent.UpdateInstanceTransform` (`self.ISM_BigHexTiles`) TileIndex (`KismetMathLibrary.MakeTransform` (.location (`InstancedStaticMeshComponent.GetInstanceTransform` (`self.ISM_BigHexTiles`) TileIndex false)) (.rotation (`InstancedStaticMeshComponent.GetInstanceTransform` (`self.ISM_BigHexTiles`) TileIndex false)) (`KismetMathLibrary.MakeVector` (.x (.scale (`InstancedStaticMeshComponent.GetInstanceTransform` (`self.ISM_BigHexTiles`) TileIndex false))) (.y (.scale (`InstancedStaticMeshComponent.GetInstanceTransform` (`self.ISM_BigHexTiles`) TileIndex false))) _returnvalue_2)) false false false)
          (`self.UpdateSmallTilesHeight` TileIndex (+ (* (.z (.scale (`InstancedStaticMeshComponent.GetInstanceTransform` (`self.ISM_BigHexTiles`) TileIndex false))) (`self.BigHexHeight`)) 1.0))
          (`self.SelectTile` TileIndex))))))

(event `UpdateSmallTilesHeight`
  (params (TileIndex :type Integer) (HeightOffset :type "Float (double-precision)"))
  (bind _returnvalue (* TileIndex 7))
  ;[0.15 0.15 0.15 0.5 72] Change height of small tiles by big tail
  (`|ExecutionSequence`
    (:`then_0`
      (for _index (range _returnvalue (+ (+ _returnvalue 6) 1))
        (`InstancedStaticMeshComponent.UpdateInstanceTransform` (`self.ISM_SmallHexTiles`) _index (`KismetMathLibrary.MakeTransform` (`KismetMathLibrary.MakeVector` (.x (.location (`InstancedStaticMeshComponent.GetInstanceTransform` (`self.ISM_SmallHexTiles`) _index false))) (.y (.location (`InstancedStaticMeshComponent.GetInstanceTransform` (`self.ISM_SmallHexTiles`) _index false))) HeightOffset) (.rotation (`InstancedStaticMeshComponent.GetInstanceTransform` (`self.ISM_SmallHexTiles`) _index false)) (.scale (`InstancedStaticMeshComponent.GetInstanceTransform` (`self.ISM_SmallHexTiles`) _index false))) false false false)))
    (:`then_1`
      (for _array_element (`.Array_3_0A781E194A4035A470EF75B61B08CBCF` (break `/Game/HexConstructor/Blueprints/Structures/SInt32Array` (`BlueprintMapLibrary.Map_Find` (`self.BigToSmallNeighbours`) TileIndex)))
        (set `self.AvgNeighbourHexesHeight` 0.0)
        (set `self.MaxNeighbourHexesHeight` 0.0)
        (bind _array (break `/Game/HexConstructor/Blueprints/Structures/SInt32Array` (`BlueprintMapLibrary.Map_Find` (`self.SmallToBigNeighbours`) _array_element)))
        (for _array_element_2 _array
          (bind _outinstancetransform (`InstancedStaticMeshComponent.GetInstanceTransform` (`self.ISM_BigHexTiles`) _array_element_2 false))
          (set `self.AvgNeighbourHexesHeight` (+ (`self.AvgNeighbourHexesHeight`) (.z (.scale _outinstancetransform))))
          (set `self.MaxNeighbourHexesHeight` (`KismetMathLibrary.FMax` (`self.MaxNeighbourHexesHeight`) (.z (.scale _outinstancetransform)))))
        (set `self.AvgNeighbourHexesHeight` (/ (`self.AvgNeighbourHexesHeight`) (`KismetArrayLibrary.Array_Length` _array)))
        (`InstancedStaticMeshComponent.UpdateInstanceTransform` (`self.ISM_SmallHexTiles`) _array_element (`KismetMathLibrary.MakeTransform` (`KismetMathLibrary.MakeVector` (.x (.location (`InstancedStaticMeshComponent.GetInstanceTransform` (`self.ISM_SmallHexTiles`) _array_element false))) (.y (.location (`InstancedStaticMeshComponent.GetInstanceTransform` (`self.ISM_SmallHexTiles`) _array_element false))) (select `bool` (== (`self.MaxNeighbourHexesHeight`) (`self.AvgNeighbourHexesHeight`)) :`false` -20000.0 :`true` (+ (* (`self.MaxNeighbourHexesHeight`) (`self.BigHexHeight`)) 1.0)))) false false false)))))

(event `SelectTile`
  (params (TileIndex :type Integer))
  (bind _returnvalue (!= TileIndex -1))
  ;[0.15 0.15 0.15 0.5 72] Select tile
  (`SceneComponent.SetVisibility` (`self.Selector`) _returnvalue true)
  (if _returnvalue
    (bind _output_get (set `self.TargetSelectorLocation` (+ (.location (`InstancedStaticMeshComponent.GetInstanceTransform` (`self.ISM_BigHexTiles`) TileIndex false)) (`KismetMathLibrary.MakeVector` 0.0 0.0 (* (.z (.scale (`InstancedStaticMeshComponent.GetInstanceTransform` (`self.ISM_BigHexTiles`) TileIndex false))) (`self.BigHexHeight`))))))
    (bind _returnvalue_2 (- _output_get (`SceneComponent.RelativeLocation` (`self.Selector`))))
    (set `self.SelectorDistance` (`KismetMathLibrary.VSize` _returnvalue_2))
    (set `self.SelectorMoveVector` (`KismetMathLibrary.Normal` _returnvalue_2))
    (set `self.SelectorTime` 0.0)))

(event `self.ReceiveTick`
  (params (DeltaSeconds :type "Float (single-precision)"))
  (set `self.SelectorTime` (+ DeltaSeconds (`self.SelectorTime`)))
  (if (< (`self.SelectorTime`) (`self.SelectorAnimationTime`))
    (`|ExecutionSequence`
      (:`then_0`
        (`SceneComponent.K2_SetRelativeLocation` (`self.Selector`) (+ (`SceneComponent.RelativeLocation` (`self.Selector`)) (* (`self.SelectorMoveVector`) (* DeltaSeconds (/ (`self.SelectorDistance`) (`self.SelectorAnimationTime`))))) false false))
      (:`then_1`
        (goto _label :!via `Reset`)))
    (else
      (`/Engine/EditorBlueprintResources/StandardMacros.DoOnce` false :!label _label
        (:`Completed`
          (`SceneComponent.K2_SetRelativeLocation` (`self.Selector`) (`self.TargetSelectorLocation`) false false))))))

(fn `GetMapHeights`
  (returns (MapHeights :type "Array of Integer"))
  (`KismetArrayLibrary.Array_Resize` (`self.Map Heights`) (`InstancedStaticMeshComponent.GetInstanceCount` (`self.ISM_BigHexTiles`)))
  (for (_ _array_index) (`self.Map Heights`)
    (`KismetArrayLibrary.Array_Set` (`self.Map Heights`) _array_index (`KismetMathLibrary.FTrunc` (.z (.scale (`InstancedStaticMeshComponent.GetInstanceTransform` (`self.ISM_BigHexTiles`) _array_index false))))))
  (return (`self.Map Heights`)))

(fn `GetSmallTileLocatin`
  (params (SmallTileIndex :type Integer))
  (returns (Location :type "Vector Structure"))
  (return (.location (`InstancedStaticMeshComponent.GetInstanceTransform` (`self.ISM_SmallHexTiles`) SmallTileIndex true))))

(fn `UserConstructionScript`)