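; Player pawn for the hex constructor: a free-moving camera with zoom and middle-mouse look that edits terrain and places buildings.
; BeginPlay finds the hex grid and building preview actors, creates the HUD and binds its mode switch.
; Tick traces under the cursor to select tiles in Landscape mode, or snap the preview and flag deletable buildings in Building mode.
; Clicks raise/lower tiles or build/delete; Q and E rotate the preview.
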(event `self.ReceiveBeginPlay`
  (bind _returnvalue (`GameplayStatics.GetPlayerController` 0))
  (`GameplayStatics.SetViewportMouseCaptureMode` "CapturePermanently_IncludingInitialMouseDown")
  (set `PlayerController.bShowMouseCursor` true _returnvalue)
  (`/Engine/EditorBlueprintResources/StandardMacros.IsValid` _returnvalue
    (:`Is Valid`
      (`EnhancedInputSubsystemInterface.AddMappingContext` (pcsubsystem `EnhancedInputLocalPlayerSubsystem` _returnvalue) "/Game/HexConstructor/Blueprints/Input/IMC_Default.IMC_Default" 0 (struct))
      (`|ExecutionSequence`
        (:`then_0`
          ; Find grid
          (bind _outactors (`GameplayStatics.GetAllActorsOfClass` "/Game/HexConstructor/Blueprints/Generator/BP_HexGridGenerator.BP_HexGridGenerator_C"))
          (if (== (`KismetArrayLibrary.Array_Length` _outactors) 1)
            (bind _output (`|GetArrayItem` _outactors))
            (`/Engine/EditorBlueprintResources/StandardMacros.IsValid` _output
              (:`Is Valid`
                (set `self.HexGrid` _output)
                ; Find building
                (bind _outactors_2 (`GameplayStatics.GetAllActorsOfClass` "/Game/HexConstructor/Blueprints/Building/BP_ShowBuilding.BP_ShowBuilding_C"))
                (if (== (`KismetArrayLibrary.Array_Length` _outactors_2) 1)
                  (bind _output_2 (`|GetArrayItem` _outactors_2))
                  (`/Engine/EditorBlueprintResources/StandardMacros.IsValid` _output_2
                    (:`Is Valid`
                      (set `self.ShowBuilding` _output_2)))
                  (else
                    (`KismetSystemLibrary.PrintString` "ERROR" true true (struct :`R` 1.0 :`A` 1.0) 2.0 "ERROR")))))
            (else
              (`KismetSystemLibrary.PrintString` "ERROR" true true (struct :`R` 1.0 :`A` 1.0) 2.0 "ERROR"))))
        (:`then_1`
          ; Create UI and change mode
          (bind _asbp_hex_grid_hud (cast `/Game/HexConstructor/Blueprints/Core/BP_HexGridHud` (`PlayerController.GetHUD` (`GameplayStatics.GetPlayerController` 0))))
          (set `self.HUD` _asbp_hex_grid_hud)
          (`/Game/HexConstructor/Blueprints/Core/BP_HexGridHud.CreateUI` (`self.HUD`))
          (add `/Game/HexConstructor/Blueprints/Core/BP_HexGridHud.ChangeMod` (`self.HUD`) (delegate `ChangeMode`)))))))

(event `ChangeMode`
  (params (Mode :type "/Game/HexConstructor/Blueprints/Enums/EMode Enum" :default "NewEnumerator0"))
  ; Create UI and change mode
  (bind _output_get (set `self.Mode` Mode))
  (`KismetSystemLibrary.PrintString` (`KismetStringLibrary.Concat_StrStr` "Current mode is: " (`|GetEnumeratorNameAsString` _output_get)) true true (struct :`G` 0.66 :`B` 1.0 :`A` 1.0) 2.0 "Mode")
  (switch `/Game/HexConstructor/Blueprints/Enums/EMode` (`self.Mode`)
    (:`NewEnumerator0`
      (`/Game/HexConstructor/Blueprints/Building/BP_ShowBuilding.SetVisibility` (`self.ShowBuilding`) false))
    (:`NewEnumerator1`
      (`/Game/HexConstructor/Blueprints/Generator/BP_HexGridGenerator.SelectTile` (`self.HexGrid`) -1))))

(event `self.ReceiveTick`
  (params (DeltaSeconds :type "Float (single-precision)"))
  (bind (_worldlocation _worlddirection) (`PlayerController.DeprojectMousePositionToWorld` (`GameplayStatics.GetPlayerController` 0)))
  (bind (_worldlocation_2 _worlddirection_2) (`PlayerController.DeprojectMousePositionToWorld` (`GameplayStatics.GetPlayerController` 0)))
  (bind _returnvalue (+ _worldlocation (* _worlddirection 10000.0)))
  (switch `/Game/HexConstructor/Blueprints/Enums/EMode` (`self.Mode`)
    (:`NewEnumerator0`
      ; Ray cast big grid tiles
      (bind _outhit (`KismetSystemLibrary.LineTraceSingle` _worldlocation_2 (+ _worldlocation_2 (* _worlddirection_2 10000.0)) "TraceTypeQuery3"))
      (bind (_bblockinghit _binitialoverlap _time _distance _location _impactpoint _normal _impactnormal _physmat _hitactor _hitcomponent _hitbonename _bonename _hititem) (`GameplayStatics.BreakHitResult` _outhit))
      (cast `/Game/HexConstructor/Blueprints/Generator/BP_HexGridGenerator` _hitactor
        (:`then`
          (if (!= _hititem (`self.TileIndex`))
            (set `self.TileIndex` _hititem)
            (`/Game/HexConstructor/Blueprints/Generator/BP_HexGridGenerator.SelectTile` (`self.HexGrid`) (`self.TileIndex`) :!label _label)))
        (:`CastFailed`
          (if (!= _hititem -1)
            (set `self.TileIndex` -1)
            (goto _label)))))
    (:`NewEnumerator1`
      ; Ray cast small grid tiles
      (`|ExecutionSequence`
        (:`then_0`
          (bind (_outhit_2 _returnvalue_2) (`KismetSystemLibrary.SphereTraceSingle` _worldlocation _returnvalue 1.0 "TraceTypeQuery3"))
          (if _returnvalue_2
            (bind _visibility (`/Game/HexConstructor/Blueprints/Building/BP_ShowBuilding.GetVisibility` (`self.ShowBuilding`)))
            (if _visibility
              (bind (_location_2 _differentheights) (`/Game/HexConstructor/Blueprints/Generator/BP_HexGridGenerator.RoundSmallTileLocation` (`self.HexGrid`) (`.Location` (`GameplayStatics.BreakHitResult` _outhit_2))))
              (if (not _differentheights)
                (if (!= _location_2 (`self.CenterTileLocation`) :`ErrorTolerance` 0.001)
                  (bind _output_get (set `self.CenterTileLocation` _location_2))
                  (`/Game/HexConstructor/Blueprints/Building/BP_ShowBuilding.UpdateLocation` (`self.ShowBuilding`) _output_get))))))
        (:`then_1`
          (bind _outhit_3 (`KismetSystemLibrary.LineTraceSingle` _worldlocation _returnvalue "TraceTypeQuery5"))
          (bind _asbp_building (cast `/Game/HexConstructor/Blueprints/Building/BP_Building` (`.HitActor` (`GameplayStatics.BreakHitResult` _outhit_3)))
            (:`then`
              (set `self.CanDelete` true)
              (set `self.BuildingToDelete` _asbp_building))
            (:`CastFailed`
              (set `self.CanDelete` false))))))))

(event `EnhancedInput|/Game/HexConstructor/Blueprints/Input/Actions/IA_Move`
  (params (ActionValue :type "Vector2D Structure") (ElapsedSeconds :type "Float (double-precision)") (TriggeredSeconds :type "Float (double-precision)") (InputAction :type "InputAction Object Reference" :default "/Game/HexConstructor/Blueprints/Input/Actions/IA_Move.IA_Move"))
  (bind _returnvalue (`GameplayStatics.GetPlayerController` 0))
  (bind (_x _y) (`KismetMathLibrary.BreakVector2D` (`KismetMathLibrary.Normal2D` (`KismetMathLibrary.MakeVector2D` ActionValue_X ActionValue_Y))))
  ; Move
  (:`Triggered`
    (`self.K2_AddActorWorldOffset` (* (+ (* _x (`self.GetActorRightVector` _returnvalue) (`GameplayStatics.GetWorldDeltaSeconds`)) (* (`KismetMathLibrary.Normal` (* (`self.GetActorForwardVector` _returnvalue) (1.0 1.0 0.0))) (`GameplayStatics.GetWorldDeltaSeconds`) _y)) (`self.MovementSpeed`) (`self.AccelerationMovement`))))
  (:`Started`
    (bind (_direction _acceleration) (`Timeline|Acceleration` :!label _label_2)
      (:`Update`
        (set `self.AccelerationMovement` _acceleration))))
  (:`Completed`
    (goto _label_2 :!via `Reverse`)))

(event `EnhancedInput|/Game/HexConstructor/Blueprints/Input/Actions/IA_Scroll`
  (params (ActionValue :type "Float (double-precision)") (ElapsedSeconds :type "Float (double-precision)") (TriggeredSeconds :type "Float (double-precision)") (InputAction :type "InputAction Object Reference" :default "/Game/HexConstructor/Blueprints/Input/Actions/IA_Scroll.IA_Scroll"))
  ; Zoom
  (:`Triggered`
    (set `SpringArmComponent.TargetArmLength` (`KismetMathLibrary.FClamp` (+ (* ActionValue 50.0) (`SpringArmComponent.TargetArmLength` (`self.SpringArm`))) 100.0 10000.0) (`self.SpringArm`))))

(event `EnhancedInput|/Game/HexConstructor/Blueprints/Input/Actions/IA_Look`
  (params (ActionValue :type "Vector2D Structure") (ElapsedSeconds :type "Float (double-precision)") (TriggeredSeconds :type "Float (double-precision)") (InputAction :type "InputAction Object Reference" :default "/Game/HexConstructor/Blueprints/Input/Actions/IA_Look.IA_Look"))
  (bind (_x _y) (`KismetMathLibrary.BreakVector2D` ActionValue))
  ; Camera rotation
  (:`Triggered`
    (if (`self.CanLook`)
      (`self.AddControllerPitchInput` _x)
      (`self.AddControllerYawInput` _y))))

(event `EnhancedInput|/Game/HexConstructor/Blueprints/Input/Actions/IA_MiddleClick`
  (params (ActionValue :type Boolean) (ElapsedSeconds :type "Float (double-precision)") (TriggeredSeconds :type "Float (double-precision)") (InputAction :type "InputAction Object Reference" :default "/Game/HexConstructor/Blueprints/Input/Actions/IA_MiddleClick.IA_MiddleClick"))
  (bind _returnvalue (`GameplayStatics.GetPlayerController` 0))
  (bind (_sizex _sizey) (`PlayerController.GetViewportSize` _returnvalue))
  ; Rotate if middle button is clicked
  (:`Triggered`
    (if ActionValue
      (`PlayerController.SetMouseLocation` _returnvalue (/ _sizex 2) (/ _sizey 2))))
  (:`Started`
    (set `PlayerController.bShowMouseCursor` false (`GameplayStatics.GetPlayerController` 0))
    (set `self.CanLook` true))
  (:`Canceled`
    (set `PlayerController.bShowMouseCursor` true (`GameplayStatics.GetPlayerController` 0))
    (set `self.CanLook` false))
  (:`Completed`
    (set `PlayerController.bShowMouseCursor` true (`GameplayStatics.GetPlayerController` 0))
    (set `self.CanLook` false)))

(event `ChangeHeight`
  (params (Scale :type "Float (double-precision)"))
  ; Change height
  (if (!= (`self.TileIndex`) -1)
    (`KismetSystemLibrary.PrintString` (`KismetStringLibrary.Concat_StrStr` "Chosen tile is: " (`KismetStringLibrary.Conv_IntToString` (`self.TileIndex`))) true true (struct :`G` 0.66 :`B` 1.0 :`A` 1.0) 3.0 "Tile")
    (`/Game/HexConstructor/Blueprints/Generator/BP_HexGridGenerator.UpdateBigTilesHeight` (`self.HexGrid`) (`self.TileIndex`) Scale)
    (else
      (`KismetSystemLibrary.PrintString` "No tiles to chose" true true (struct :`G` 0.66 :`B` 1.0 :`A` 1.0) 3.0 "Tile"))))

(event `EnhancedInput|/Game/HexConstructor/Blueprints/Input/Actions/IA_LeftClick`
  (params (ActionValue :type Boolean) (ElapsedSeconds :type "Float (double-precision)") (TriggeredSeconds :type "Float (double-precision)") (InputAction :type "InputAction Object Reference" :default "/Game/HexConstructor/Blueprints/Input/Actions/IA_LeftClick.IA_LeftClick"))
  ; LMB
  (:`Triggered`
    (if ActionValue
      (`KismetSystemLibrary.Delay` (`KismetMathLibrary.FMax` (`GameplayStatics.GetWorldDeltaSeconds`) 0.05))
      (switch `/Game/HexConstructor/Blueprints/Enums/EMode` (`self.Mode`)
        (:`NewEnumerator0`
          (`self.ChangeHeight` 1.0 :!label _label_3)))))
  (:`Canceled`
    (switch `/Game/HexConstructor/Blueprints/Enums/EMode` (`self.Mode`)
      (:`NewEnumerator0`
        (goto _label_3))
      (:`NewEnumerator1`
        (`/Game/HexConstructor/Blueprints/Building/BP_ShowBuilding.Build` (`self.ShowBuilding`))))))

(event `EnhancedInput|/Game/HexConstructor/Blueprints/Input/Actions/IA_RightClick`
  (params (ActionValue :type Boolean) (ElapsedSeconds :type "Float (double-precision)") (TriggeredSeconds :type "Float (double-precision)") (InputAction :type "InputAction Object Reference" :default "/Game/HexConstructor/Blueprints/Input/Actions/IA_RightClick.IA_RightClick"))
  ; RMB
  (:`Triggered`
    (if ActionValue
      (`KismetSystemLibrary.Delay` (`KismetMathLibrary.FMax` (`GameplayStatics.GetWorldDeltaSeconds`) 0.05))
      (switch `/Game/HexConstructor/Blueprints/Enums/EMode` (`self.Mode`)
        (:`NewEnumerator0`
          (`self.ChangeHeight` -1.0 :!label _label_4)))))
  (:`Canceled`
    (switch `/Game/HexConstructor/Blueprints/Enums/EMode` (`self.Mode`)
      (:`NewEnumerator0`
        (goto _label_4))
      (:`NewEnumerator1`
        (if (`self.CanDelete`)
          (`/Game/HexConstructor/Blueprints/Building/BP_ShowBuilding.DeleteBuilding` (`self.ShowBuilding`) (`self.BuildingToDelete`)))))))

(event `EnhancedInput|/Game/HexConstructor/Blueprints/Input/Actions/IA_Q`
  (params (ActionValue :type Boolean) (ElapsedSeconds :type "Float (double-precision)") (TriggeredSeconds :type "Float (double-precision)") (InputAction :type "InputAction Object Reference" :default "/Game/HexConstructor/Blueprints/Input/Actions/IA_Q.IA_Q"))
  (:`Started`
    (switch `/Game/HexConstructor/Blueprints/Enums/EMode` (`self.Mode`)
      (:`NewEnumerator1`
        (bind _visibility (`/Game/HexConstructor/Blueprints/Building/BP_ShowBuilding.GetVisibility` (`self.ShowBuilding`)))
        (if _visibility
          (`/Game/HexConstructor/Blueprints/Building/BP_ShowBuilding.UpdateRotation` (`self.ShowBuilding`) -60.0 (`self.CenterTileLocation`)))))))

(event `EnhancedInput|/Game/HexConstructor/Blueprints/Input/Actions/IA_E`
  (params (ActionValue :type Boolean) (ElapsedSeconds :type "Float (double-precision)") (TriggeredSeconds :type "Float (double-precision)") (InputAction :type "InputAction Object Reference" :default "/Game/HexConstructor/Blueprints/Input/Actions/IA_E.IA_E"))
  (:`Started`
    (switch `/Game/HexConstructor/Blueprints/Enums/EMode` (`self.Mode`)
      (:`NewEnumerator1`
        (bind _visibility (`/Game/HexConstructor/Blueprints/Building/BP_ShowBuilding.GetVisibility` (`self.ShowBuilding`)))
        (if _visibility
          (`/Game/HexConstructor/Blueprints/Building/BP_ShowBuilding.UpdateRotation` (`self.ShowBuilding`) 60.0 (`self.CenterTileLocation`)))))))

(fn `UserConstructionScript`)