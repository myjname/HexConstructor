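; Game mode for a hex grid constructor that owns saving and loading of the terrain and placed buildings.
; On BeginPlay it forces default display settings and finds the single BP_HexGridGenerator.
; It then loads or creates the first-slot BP_Save, generates the grid from size and heights, and respawns any saved buildings.
; SaveTo gathers building actors and, for existing slots, current generator heights, then writes the named slot.
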(event `self.ReceiveBeginPlay`
  (bind (_x _y) (break `IntPoint` (`self.Grid Size`)))
  (`|ExecutionSequence`
    (:`then_0`
      ; Default settings
      (bind _returnvalue (`GameUserSettings.GetGameUserSettings`))
      (`GameUserSettings.SetOverallScalabilityLevel` _returnvalue 3)
      (`GameUserSettings.SetOverallScalabilityLevel` _returnvalue 3)
      (`GameUserSettings.SetResolutionScaleValueEx` _returnvalue 100.0)
      (`GameUserSettings.SetFullscreenMode` _returnvalue "Windowed")
      (`GameUserSettings.SetScreenResolution` _returnvalue (make `IntPoint` 1920 1080))
      (`GameUserSettings.ApplySettings` _returnvalue true))
    (:`then_1`
      (bind _outactors (`GameplayStatics.GetAllActorsOfClass` "/Game/HexConstructor/Blueprints/Generator/BP_HexGridGenerator.BP_HexGridGenerator_C"))
      (if (== (`KismetArrayLibrary.Array_Length` _outactors) 1)
        (set `self.HexGridGenerator` (`|GetArrayItem` _outactors))
        (set `self.Initial Height` (`/Game/HexConstructor/Blueprints/Generator/BP_HexGridGenerator.InitialHeight` (`self.HexGridGenerator`)))
        (else
          (`KismetSystemLibrary.PrintString` "ERROR" true true (struct :`R` 1.0 :`A` 1.0) 10.0 "ERROR"))))
    (:`then_2`
      (bind _returnvalue_2 (`GameplayStatics.DoesSaveGameExist` (`self.FirstSlotName`)))
      (if _returnvalue_2
        (bind _returnvalue_3 (`GameplayStatics.LoadGameFromSlot` (`self.FirstSlotName`)))
        (bind _asbp_save (cast `/Game/HexConstructor/Blueprints/Save/BP_Save` _returnvalue_3))
        (set `self.Save` _asbp_save)
        (bind _output_get (set `self.SaveVersion` (`/Game/HexConstructor/Blueprints/Save/BP_Save.Version` (`self.Save`))))
        (`KismetSystemLibrary.PrintString` (select `bool` (`KismetStringLibrary.IsEmpty` _output_get) :`false` (`KismetStringLibrary.Concat_StrStr` "Game version: " _output_get) :`true` "No game version in save") true true (struct :`R` 1.0 :`G` 0.309595 :`A` 1.0) 5.0 "GAMEVERSION")
        (set `self.MapHeights` (`/Game/HexConstructor/Blueprints/Save/BP_Save.MapHeights` (`self.Save`)))
        (set `self.Grid Size` (`/Game/HexConstructor/Blueprints/Save/BP_Save.GridSize` (`self.Save`)))
        (`/Game/HexConstructor/Blueprints/Generator/BP_HexGridGenerator.GenerateHexGrid` (`self.HexGridGenerator`) (`self.Grid Size`) (`self.MapHeights`))
        (set `self.Buildings` (`/Game/HexConstructor/Blueprints/Save/BP_Save.Buildings` (`self.Save`)))
        (if (> (`KismetArrayLibrary.Array_Length` (`self.Buildings`)) 0)
          (for _array_element (`self.Buildings`)
            (bind (_building_id _transform _color) (break `/Game/HexConstructor/Blueprints/Structures/SSaveBuilding` _array_element))
            (`|SpawnActorFromClass` "/Game/HexConstructor/Blueprints/Building/BP_Building.BP_Building_C" _transform "Undefined" "MultiplyWithRoot" null _color _building_id null)))
        (else
          ;[0.15 0.15 0.15 0.5 72] Create save if save does not exist
          (`|ExecutionSequence`
            (:`then_0`
              (`KismetArrayLibrary.Array_Resize` (`self.MapHeights`) (* _x _y))
              (for (_ _array_index) (`self.MapHeights`)
                (`KismetArrayLibrary.Array_Set` (`self.MapHeights`) _array_index (`KismetMathLibrary.FTrunc` (`self.Initial Height`)))))
            (:`then_1`
              (`self.CreateSave` (`self.InitialSaveVersion`) (`self.Grid Size`) (`self.MapHeights`) (`self.Buildings`) (`self.FirstSlotName`))
              (`/Game/HexConstructor/Blueprints/Generator/BP_HexGridGenerator.GenerateHexGrid` (`self.HexGridGenerator`) (`self.Grid Size`) (`self.MapHeights`)))))))))

(event `CreateSave`
  (params (GameVersion :type String) (GridSize :type "IntPoint Structure") (MapHeights :type "Array of Integer") (Buildings :type "Array of /Game/HexConstructor/Blueprints/Structures/SSaveBuilding Structure") (SaveName :type String))
  ;[0.15 0.15 0.15 0.5 72] Create save
  (bind _returnvalue (`GameplayStatics.CreateSaveGameObject` "/Game/HexConstructor/Blueprints/Save/BP_Save.BP_Save_C"))
  (set `self.Save` _returnvalue)
  (set `self.SaveVersion` GameVersion)
  (set `/Game/HexConstructor/Blueprints/Save/BP_Save.GridSize` GridSize (`self.Save`))
  (set `/Game/HexConstructor/Blueprints/Save/BP_Save.MapHeights` MapHeights (`self.Save`))
  (set `/Game/HexConstructor/Blueprints/Save/BP_Save.Buildings` Buildings (`self.Save`))
  (`GameplayStatics.SaveGameToSlot` (`self.Save`) SaveName))

(event `SaveTo`
  (params (SaveName :type String))
  (set `self.Save Name` SaveName)
  (`|ExecutionSequence`
    (:`then_0`
      (`KismetArrayLibrary.Array_Clear` (`self.Buildings`))
      (bind _outactors (`GameplayStatics.GetAllActorsOfClass` "/Game/HexConstructor/Blueprints/Building/BP_Building.BP_Building_C"))
      (set `self.BuildingActors` _outactors)
      (`KismetArrayLibrary.Array_Resize` (`self.Buildings`) (`KismetArrayLibrary.Array_Length` (`self.BuildingActors`)))
      (for (_array_element _array_index) (`self.BuildingActors`)
        (`KismetArrayLibrary.Array_Set` (`self.Buildings`) _array_index (make `/Game/HexConstructor/Blueprints/Structures/SSaveBuilding` (`/Game/HexConstructor/Blueprints/Building/BP_Building.Building_ID` _array_element) (`self.GetTransform` _array_element) (`/Game/HexConstructor/Blueprints/Building/BP_Building.BuildingColor` _array_element)))))
    (:`then_1`
      (bind _returnvalue (`GameplayStatics.DoesSaveGameExist` (`self.Save Name`)))
      (if _returnvalue
        (bind _returnvalue_2 (`GameplayStatics.LoadGameFromSlot` (`self.Save Name`)))
        (bind _asbp_save (cast `/Game/HexConstructor/Blueprints/Save/BP_Save` _returnvalue_2))
        (set `self.Save` _asbp_save)
        (set `/Game/HexConstructor/Blueprints/Save/BP_Save.GridSize` (`self.Grid Size`) (`self.Save`))
        (bind _mapheights (`/Game/HexConstructor/Blueprints/Generator/BP_HexGridGenerator.GetMapHeights` (`self.HexGridGenerator`)))
        (set `/Game/HexConstructor/Blueprints/Save/BP_Save.MapHeights` _mapheights (`self.Save`))
        (set `/Game/HexConstructor/Blueprints/Save/BP_Save.Buildings` (`self.Buildings`) (`self.Save`))
        (set `/Game/HexConstructor/Blueprints/Save/BP_Save.Version` (`self.InitialSaveVersion`) (`self.Save`))
        (`GameplayStatics.SaveGameToSlot` (`self.Save`) (`self.Save Name`))
        (else
          (`self.CreateSave` (`self.InitialSaveVersion`) (`self.Grid Size`) (`self.MapHeights`) (`self.Buildings`) (`self.Save Name`)))))))

(fn `UserConstructionScript`)