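; Placement preview actor for hex-grid buildings that shows the selected mesh, validates the spot and spawns BP_Building.
; The building's data asset supplies the mesh and small-tile footprint, converted to offsets that rotate with the preview.
; Per-tile traces detect existing buildings and read grid heights, snapping the preview just above the highest tile.
; CanBuild requires level, unoccupied ground and drives the material through custom primitive data, refreshing after moves, rotations, builds and deletions.
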(event `self.ReceiveBeginPlay`
  (set `self.SmallTileRadius` (/ (`self.TileRadius`) 3.0))
  (set `self.SmallTileOffset` (* (`self.SmallTileRadius`) (`KismetMathLibrary.DegSin` 60.0)))
  ; Find grid
  (bind _outactors (`GameplayStatics.GetAllActorsOfClass` "/Game/HexConstructor/Blueprints/Generator/BP_HexGridGenerator.BP_HexGridGenerator_C"))
  (if (== (`KismetArrayLibrary.Array_Length` _outactors) 1)
    (bind _output (`|GetArrayItem` _outactors))
    (`/Engine/EditorBlueprintResources/StandardMacros.IsValid` _output
      (:`Is Valid`
        (set `self.HexGrid` _output)))
    (else
      (`KismetSystemLibrary.PrintString` "ERROR" true true (struct :`R` 1.0 :`A` 1.0) 2.0 "ERROR"))))

(event `UpdateVisual`
  (params (Building_ID :type Name))
  ; Update visual
  (bind _output_get (set `self.Building ID` Building_ID))
  (bind _returnvalue (`|GetDataTableRow` "/Game/HexConstructor/Blueprints/DataTables/DT_BuildingIDs.DT_BuildingIDs" _output_get)
    (:`then`
      (bind _output_get_2 (set `self.DA_Building` (`.DataAsset_3_558CC024432CAA6C2D297B868A6AEBC9` (break `/Game/HexConstructor/Blueprints/Structures/SBuildingID` _returnvalue))))
      (`/Engine/EditorBlueprintResources/StandardMacros.IsValid` _output_get_2
        (:`Is Valid`
          (`self.K2_SetActorRotation` (struct))
          (`|ExecutionSequence`
            (:`then_0`
              (`StaticMeshComponent.SetStaticMesh` (`self.Building`) (`.Mesh_4_3D76750A4EF1A02CF262638069B61282` (break `/Game/HexConstructor/Blueprints/Structures/SBuilding` (`/Game/HexConstructor/Blueprints/DataAssets/Building/Data/PDA_Building.Building` (`self.DA_Building`))))))
            (:`then_1`
              (`KismetArrayLibrary.Array_Clear` (`self.TilesOffsets`))
              (for _array_element (`.Tiles_21_FD8E6C894E1DD852ADAAF8B1F77E42E3` (break `/Game/HexConstructor/Blueprints/Structures/SBuilding` (`/Game/HexConstructor/Blueprints/DataAssets/Building/Data/PDA_Building.Building` (`self.DA_Building`))))
                (bind _returnvalue_2 (* (`self.SmallTileOffset`) (`.X` (break `IntPoint` _array_element))))
                (bind ((`Y` _y)) (break `IntPoint` _array_element))
                (`KismetArrayLibrary.Array_Add` (`self.TilesOffsets`) (`KismetMathLibrary.MakeVector` (select `bool` (!= (mod _y 2) 0) :`false` _returnvalue_2 :`true` (+ _returnvalue_2 (/ (`self.SmallTileOffset`) 2.0))) (* (* (`self.SmallTileRadius`) 0.75) _y)))))))))))

(event `UpdateLocation`
  (params (CenterTileLocation :type "Vector Structure"))
  ; Update location
  (set `self.Center Tile Location` CenterTileLocation)
  (`|ExecutionSequence`
    (:`then_0`
      (set `self.SmallTilesMaxHeight` 0.0)
      (set `self.SmallTilesAvrHeight` 0.0)
      (set `self.TraceNotEqual` false)
      (set `self.TraceHitBuilding` false)
      (set `self.Different Heights` false)
      (for _array_element (`self.TilesOffsets`)
        (bind _returnvalue (+ _array_element CenterTileLocation))
        (bind _returnvalue_2 (+ _returnvalue (0.0 0.0 5000.0)))
        (bind _returnvalue_3 (- _returnvalue (0.0 0.0 1000.0)))
        (bind (_outhit _returnvalue_4) (`KismetSystemLibrary.SphereTraceSingle` :`Start` _returnvalue_2 :`End` _returnvalue_3 :`Radius` 1.0 :`TraceChannel` "TraceTypeQuery3" :`DrawTime` 0.3))
        (set `self.Out Hit` _outhit)
        (set `self.TraceResult1` _returnvalue_4)
        (bind (_outhit_2 _returnvalue_5) (`KismetSystemLibrary.LineTraceSingle` :`Start` _returnvalue_2 :`End` _returnvalue_3 :`TraceChannel` "TraceTypeQuery5" :`DrawDebugType` "ForDuration" :`DrawTime` 0.3))
        (set `self.TraceResult2` _returnvalue_5)
        (set `self.TraceHitBuilding` (or (`self.TraceResult2`) (`self.TraceHitBuilding`)))
        (if (and (not (`self.TraceResult2`)) (`self.TraceResult1`))
          (bind (_location _differentheights) (`/Game/HexConstructor/Blueprints/Generator/BP_HexGridGenerator.RoundSmallTileLocation` (`self.HexGrid`) (`.Location` (`GameplayStatics.BreakHitResult` (`self.Out Hit`))) :!label _label))
          (set `self.Different Heights` (or _differentheights (`self.Different Heights`)))
          (bind _z (.z _location))
          (set `self.SmallTilesMaxHeight` (`KismetMathLibrary.FMax` _z (`self.SmallTilesMaxHeight`)))
          (set `self.SmallTilesAvrHeight` (+ _z (`self.SmallTilesAvrHeight`)))
          (set `self.TraceNotEqual` true)))
      (if (not (`self.TraceNotEqual`))
        (goto _label)))
    (:`then_1`
      (set `self.SmallTilesAvrHeight` (/ (`self.SmallTilesAvrHeight`) (`KismetArrayLibrary.Array_Length` (`self.TilesOffsets`))))
      (`self.K2_SetActorLocation` (`KismetMathLibrary.MakeVector` (.x CenterTileLocation) (.y CenterTileLocation) (+ (`self.SmallTilesMaxHeight`) 2.0)))
      (bind _output_get (set `self.CanBuild` (and (== (`self.SmallTilesAvrHeight`) (`self.SmallTilesMaxHeight`)) (not (`self.TraceHitBuilding`)) (not (`self.Different Heights`)))))
      (`PrimitiveComponent.SetCustomPrimitiveDataFloat` (`self.Building`) 0 (select `bool` _output_get :`true` 1.0)))))

(event `self.ReceiveTick`
  (params (DeltaSeconds :type "Float (single-precision)")))

(event `UpdateRotation`
  (params (Angle :type "Float (double-precision)") (CenterTileLocation :type "Vector Structure"))
  ; Update rotation
  (for (_array_element _array_index) (`self.TilesOffsets`)
    (`KismetArrayLibrary.Array_Set` (`self.TilesOffsets`) _array_index (`KismetMathLibrary.RotateAngleAxis` _array_element Angle (0.0 0.0 1.0))))
  (`self.K2_SetActorRotation` (`KismetMathLibrary.ComposeRotators` (`self.K2_GetActorRotation`) (`KismetMathLibrary.MakeRotator` 0.0 0.0 Angle)))
  (`self.UpdateLocation` CenterTileLocation))

(event `Build`
  ; Build
  (if (`self.CanBuild`)
    (`|SpawnActorFromClass` "/Game/HexConstructor/Blueprints/Building/BP_Building.BP_Building_C" (`self.GetTransform`) "Undefined" "MultiplyWithRoot" null (`self.Building Color`) (`self.Building ID`) null)
    (`self.UpdateLocation` (`self.Center Tile Location`))))

(event `DeleteBuilding`
  (params (Building :type "/Game/HexConstructor/Blueprints/Building/BP_Building Object Reference"))
  ; Delete building
  (`self.K2_DestroyActor` Building)
  (`self.UpdateLocation` (`self.Center Tile Location`)))

(fn `GetVisibility`
  (returns (Visibility :type Boolean))
  (return (`SceneComponent.bVisible` (`self.DefaultSceneRoot`))))

(fn `SetVisibility`
  (params (NewVisibility :type Boolean))
  (`SceneComponent.SetVisibility` (`self.DefaultSceneRoot`) NewVisibility true))

(fn `UserConstructionScript`)