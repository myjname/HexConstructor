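; BP_Building is a data-driven building actor for HexConstructor that takes its look from a BuildingID and a BuildingColor.
; The construction script finds the BuildingID row in DT_BuildingIDs and applies the mesh and material from that row's data asset.
; It writes the color into Custom Primitive Data on the static mesh, allowing per-building tint without dynamic material instances.
; The event graph holds no active logic.
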(fn `UserConstructionScript`
  (bind (_buildingcolor_r _buildingcolor_g _buildingcolor_b _buildingcolor_a) (break `LinearColor` (`self.BuildingColor`)))
  (bind _returnvalue (`|GetDataTableRow` "/Game/HexConstructor/Blueprints/DataTables/DT_BuildingIDs.DT_BuildingIDs" (`self.Building_ID`))
    (:`then`
      (bind ((`Mesh_4_3D76750A4EF1A02CF262638069B61282` _mesh) (`Material_22_B77D205946685C8F017DE3B705C3EEE8` _material)) (break `/Game/HexConstructor/Blueprints/Structures/SBuilding` (`/Game/HexConstructor/Blueprints/DataAssets/Building/Data/PDA_Building.Building` (`.DataAsset_3_558CC024432CAA6C2D297B868A6AEBC9` (break `/Game/HexConstructor/Blueprints/Structures/SBuildingID` _returnvalue)))))
      (`StaticMeshComponent.SetStaticMesh` (`self.StaticMesh`) _mesh)
      (`GeometryScriptLibrary_SceneUtilityFunctions.SetComponentMaterialList` (`self.StaticMesh`) (`|MakeArray` _material) null)
      (`PrimitiveComponent.SetCustomPrimitiveDataVector4` (`self.StaticMesh`) 0 (`KismetMathLibrary.MakeVector4` _buildingcolor_r _buildingcolor_g _buildingcolor_b _buildingcolor_a)))))